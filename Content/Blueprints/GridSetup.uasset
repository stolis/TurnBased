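; GridSetup is an actor that computes a hexagonal tile layout around the player's character on BeginPlay.
; GenerateGrid builds unit hex coordinates from Radius, which BeginPlay scales and offsets by the capsule location into WsCoordinates, then prints the count.
; A bound RestartGrid event moves the actor's root to a new center.
; GridBase spawning, instancing, edge-tile coloring and per-tile repositioning are disconnected, and DestroyGrid is never called.
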(event Custom|RestartGrid
  (params (NewGridCenter :type Vector))
  (Transformation|SetWorldLocation (Variables|Default|GetDefaultSceneRoot) NewGridCenter false false))

(event EventBeginPlay
  (EventDispatchers|BindEventtoRestartGridEvent (delegate Custom|RestartGrid))
  (Utilities|GenerateGrid
    (:Out
      (for _index (range 0 (- (Utilities|Array|Length (Variables|Default|GettileCoordinates)) 1))
        (Variables|Default|SetIndex _index)
        (bind _astop_down_character (Utilities|Casting|CastToTopDownCharacter (Game|Player|GetPlayerPawn 0)))
        (Variables|Default|SetTopDownCharacter _astop_down_character)
        (Utilities|Array|Add (Variables|Default|GetwsCoordinates) (Math|Vector|MakeVector (+ (* (.x (Utilities|Array|Get(acopy) (Variables|Default|GettileCoordinates) _index)) 187.0) (.x (Transformation|GetWorldLocation (Variables|/Script/Engine.Character|GetCapsuleComponent (Variables|Default|GetTopDownCharacter))))) (+ (* (.y (Utilities|Array|Get(acopy) (Variables|Default|GettileCoordinates) _index)) 187.0) (.y (Transformation|GetWorldLocation (Variables|/Script/Engine.Character|GetCapsuleComponent (Variables|Default|GetTopDownCharacter))))) 0.0)))
      (Development|PrintString (Utilities|String|ToString(Integer) (Utilities|Array|Length (Variables|Default|GetwsCoordinates)))))))

(event Collision|EventActorBeginOverlap
  (params (OtherActor :type Actor%20Object%20Reference)))

(event EventTick
  (params (DeltaSeconds :type Float%20%28single-precision%29)))

(fn ConstructionScript)