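; GridBase is the clickable tile grid for top-down play, drawn as hierarchical instanced meshes with a decal at each tile.
; A GenerateGrid event, bound on BeginPlay, adds both from supplied coordinates.
; Releasing on GridTile sends its location to TopDownController; overlap on that clicked tile restarts GridSetup's grid after a short delay.
; Instance hover only prints an overlapping component's name, as glow and dynamic-material logic is disconnected.
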(event OnBeginCursorOver(GridTile)
  (params (TouchedComponent :type Primitive%20Component%20Object%20Reference)))

(event OnEndCursorOver(GridTile)
  (params (TouchedComponent :type Primitive%20Component%20Object%20Reference)))

(event OnBeginCursorOver(HierarchicalInstancedStaticMesh)
  (params (TouchedComponent :type Primitive%20Component%20Object%20Reference))
  (bind _ashierarchical_instanced_static_mesh_component (Utilities|Casting|CastToHierarchicalInstancedStaticMeshComponent TouchedComponent))
  (Development|PrintString (Utilities|GetDisplayName (Utilities|Array|Get(acopy) (Class|PrimitiveComponent|GetOverlappingComponents _ashierarchical_instanced_static_mesh_component)))))

(event OnComponentBeginOverlap(GridTile)
  (params (OverlappedComponent :type Primitive%20Component%20Object%20Reference) (OtherActor :type Actor%20Object%20Reference) (OtherComp :type Primitive%20Component%20Object%20Reference) (OtherBodyIndex :type Integer) (bFromSweep :type Boolean) (SweepResult :type Hit%20Result%20Structure%20%28by%20ref%29))
  (if (== OverlappedComponent (Variables|Default|GetClickedTile))
    (Utilities|FlowControl|Delay 0.5)
    (bind _outactors (Actor|GetAllActorsOfClass "/Game/Blueprints/GridSetup.GridSetup_C"))
    (Default|CallRestartGridEvent (Utilities|Array|Get(acopy) _outactors) (Transformation|GetWorldLocation (Variables|/Game/Blueprints/GridSetup.GridSetup_C|GetDefaultSceneRoot (Utilities|Array|Get(acopy) _outactors))))))

(event OnReleased(GridTile)
  (params (TouchedComponent :type Primitive%20Component%20Object%20Reference) (ButtonReleased :type Key%20Structure))
  (bind _output_get (Variables|Default|SetClickedTile TouchedComponent))
  (Variables|Default|SetSelectedGridTileLoc (Transformation|GetWorldLocation _output_get))
  (bind _astop_down_controller (Utilities|Casting|CastToTopDownController (Game|GetPlayerController 0)))
  (Default|CallMouseReleasedEvent _astop_down_controller (Variables|Default|GetSelectedGridTileLoc)))

(event Custom|GenerateGrid
  (params (wsCoordinates :type Array%20of%20Vectors))
  (for _array_element wsCoordinates
    (Components|InstancedStaticMesh|AddInstance (Variables|Default|GetHierarchicalInstancedStaticMesh) (Math|Transform|MakeTransform _array_element "0, 0, 0" "1,1,1"))
    (AddComponent|AddDecalComponent false (Math|Transform|MakeTransform _array_element "90.000000, 0,90.000000" "1,1,1"))))

(event EventBeginPlay
  (EventDispatchers|BindEventtoAddInstance (delegate Custom|GenerateGrid)))

(event Collision|EventActorBeginOverlap
  (params (OtherActor :type Actor%20Object%20Reference)))

(event EventTick
  (params (DeltaSeconds :type Float%20%28single-precision%29)))

(fn ConstructionScript)